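; BP_DoorBluetooth is a door actor that swings open and closed when its OpenCloseDoor event is called.
; BeginPlay sets the target rotation to a quarter turn, with InvertRotation choosing the direction.
; Each call alternates through a FlipFlop between playing and reversing the DoorAnimation timeline, whose alpha interpolates the door mesh's relative rotation toward that target.
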(event Custom|OpenCloseDoor
  (Utilities|FlowControl|FlipFlop
    (:A
      (bind _alpha (Timeline|Door%20Animation Play)
        (:Update
          (Transformation|SetRelativeRotation (Variables|Default|GetDoor_Door_GEO) (Math|Rotator|Lerp(Rotator) "0, 0, 0" (Variables|Default|GetDoor%20Rotation) _alpha) false false))))
    (:B
      (Timeline|Door%20Animation Reverse))))

(event EventBeginPlay
  (if (Variables|Default|GetInvertRotation)
    (Variables|Default|SetDoor%20Rotation "0.000000,90.000000,0.000000")
    (else
      (Variables|Default|SetDoor%20Rotation "0.000000,-90.000000,0.000000"))))

(fn ConstructionScript)