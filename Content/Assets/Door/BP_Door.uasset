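; BP_Door is an interactable door that the player opens and closes with the interact input.
; On BeginPlay it enables input for player controller 0, and overlap events open and close a Gate so IA_interact only works while an actor overlaps it.
; Each accepted press alternates through a FlipFlop between playing and reversing the DoorAnimation timeline, which lerps the door mesh's relative rotation to swing it 90 degrees.
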(event Input|EnhancedActionEvents|EnhancedInputActionIA_interact
  (params (ActionValue :type Boolean) (ElapsedSeconds :type Float%20%28double-precision%29) (TriggeredSeconds :type Float%20%28double-precision%29) (InputAction :type Input%20Action%20Object%20Reference :default "/Game/ThirdPerson/Input/Actions/IA_interact.IA_interact"))
  (:Started
    (Utilities|FlowControl|Gate true
      (:Exit
        (Utilities|FlowControl|FlipFlop
          (:A
            (bind _alpha (Timeline|Door%20Animation Play)
              (:Update
                (Transformation|SetRelativeRotation (Variables|Default|GetDoor_Door_GEO) (Math|Rotator|Lerp(Rotator) "0, 0, 0" "0.000000,-90.000000,0.000000" _alpha) false false))))
          (:B
            (Timeline|Door%20Animation Reverse)))))))

(event EventBeginPlay
  (Input|EnableInput (Game|GetPlayerController 0)))

(event Collision|EventActorBeginOverlap
  (params (OtherActor :type Actor%20Object%20Reference))
  (Utilities|FlowControl|Gate true) ; enters at Open
)

(event EventTick
  (params (DeltaSeconds :type Float%20%28single-precision%29)))

(event Collision|EventActorEndOverlap
  (params (OtherActor :type Actor%20Object%20Reference))
  (Utilities|FlowControl|Gate true) ; enters at Close
)

(fn ConstructionScript)